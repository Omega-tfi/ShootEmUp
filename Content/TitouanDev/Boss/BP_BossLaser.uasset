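; Boss laser attack actor that follows BP_Boss at a fixed offset and damages the player character on overlap.
; After a start delay, it repeatedly picks at random between an aimed shot and a fixed straight shot, with random pauses.
; Timelines scale a telegraph cylinder and a damage cylinder, whose collision and sound switch on once the beam widens.
; Aimed shots face the ship position captured when the attack starts.
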(event Custom|TargetAndShoot
  (bind _damagecylinder (Variables|Default|GetDamageCylinder))
  (bind _asbp_main_chara (Utilities|Casting|CastToBP_MainChara (Game|GetPlayerCharacter 0)))
  (Variables|Default|SetTarget (Transformation|GetWorldLocation (Variables|/Game/TitouanDev/BP_MainChara.BP_MainChara_C|GetShip _asbp_main_chara)))
  (bind (_direction _targetsize _lasersize) (Timeline|Timeline PlayFromStart)
    (:Update
      (Transformation|SetRelativeScale3D (Variables|Default|GetTargetCylinder) (Math|Vector|MakeVector _targetsize _targetsize 5e+01))
      (Transformation|SetRelativeScale3D (Variables|Default|GetDamageCylinder) (Math|Vector|MakeVector _lasersize _lasersize 5e+01))
      (Transformation|SetActorRotation (Math|Rotator|FindLookatRotation (- (Transformation|GetActorLocation (Variables|Default|GetBoss_Ref)) "0.000000,1000.000000,0.000000") (Variables|Default|GetTarget)))
      (if (>= _lasersize 0.1)
        (Utilities|FlowControl|DoOnce false :!label _label
          (:Completed
            (Collision|SetCollisionEnabled _damagecylinder "QueryOnly")
            (Audio|PlaySound2D "/Game/SFX/SoundCues/SC_Laser.SC_Laser" 0.5 1.0 0.0 0 0)))
        (else
          (Collision|SetCollisionEnabled _damagecylinder "NoCollision"))))
    (:Finished
      (Utilities|FlowControl|Delay (+ (* (Math|Random|RandomFloat) 2.0) 1.0))
      (if (Math|Random|RandomBool)
        (CallFunction|TargetandShoot)
        (goto _label Reset)
        (else
          (CallFunction|ShootStraight)
          (goto _label Reset))))))

(event Custom|ShootStraight
  (bind _damagecylinder (Variables|Default|GetDamageCylinder))
  (bind _asbp_main_chara (Utilities|Casting|CastToBP_MainChara (Game|GetPlayerCharacter 0)))
  (Variables|Default|SetTarget (Transformation|GetWorldLocation (Variables|/Game/TitouanDev/BP_MainChara.BP_MainChara_C|GetShip _asbp_main_chara)))
  (bind (_direction _targetsize _lasersize) (Timeline|Timeline_0 PlayFromStart)
    (:Update
      (Transformation|SetRelativeScale3D (Variables|Default|GetTargetCylinder) (Math|Vector|MakeVector _targetsize _targetsize 5e+01))
      (Transformation|SetRelativeScale3D (Variables|Default|GetDamageCylinder) (Math|Vector|MakeVector _lasersize _lasersize 5e+01))
      (Transformation|SetActorRotation "0.000000,-90.000000,0.000000")
      (if (>= _lasersize 0.1)
        (Utilities|FlowControl|DoOnce false :!label _label
          (:Completed
            (Collision|SetCollisionEnabled _damagecylinder "QueryOnly")
            (Audio|PlaySound2D "/Game/SFX/SoundCues/SC_Laser.SC_Laser" 0.5 1.0 0.0 0 0)))
        (else
          (Collision|SetCollisionEnabled _damagecylinder "NoCollision"))))
    (:Finished
      (Utilities|FlowControl|Delay (+ (* (Math|Random|RandomFloat) 2.0) 1.0))
      (if (Math|Random|RandomBool)
        (CallFunction|TargetandShoot)
        (goto _label Reset)
        (else
          (CallFunction|ShootStraight)
          (goto _label Reset))))))

(event EventBeginPlay
  (bind _returnvalue (Actor|GetActorOfClass "/Game/TitouanDev/Boss/BP_Boss.BP_Boss_C"))
  (Variables|Default|SetBoss_Ref _returnvalue)
  (Utilities|FlowControl|Delay 2.0)
  (if (Math|Random|RandomBool)
    (CallFunction|TargetandShoot)
    (else
      (CallFunction|ShootStraight))))

(event Collision|EventActorBeginOverlap
  (params (OtherActor :type Actor%20Object%20Reference))
  (bind _asbp_main_chara (Utilities|Casting|CastToBP_MainChara OtherActor))
  (Game|Damage|ApplyDamage _asbp_main_chara 3.0 0 0))

(event EventTick
  (params (DeltaSeconds :type Float%20%28single-precision%29))
  (Transformation|SetActorLocation (- (Transformation|GetActorLocation (Variables|Default|GetBoss_Ref)) "0.000000,1000.000000,0.000000") false false))

(fn ConstructionScript)