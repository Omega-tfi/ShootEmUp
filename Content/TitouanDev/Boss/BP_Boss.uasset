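; BP_Boss is a boss that wakes when the player comes within range, spawning a laser and health bar.
; A self-restarting timeline moves it along X while it keeps a fixed Y lead on the player, and a looping timer spawns secondary-shot spawners at a random cannon.
; Overlap damages the player.
; At zero life it removes the laser, staggers explosion particles, hides its mesh and opens the win level.
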(event Custom|Death
  (Variables|Default|SetDead? true)
  (bind _returnvalue (Actor|GetActorOfClass "/Game/TitouanDev/Boss/BP_BossLaser.BP_BossLaser_C"))
  (Utilities|IsValid _returnvalue
    (:Is%20Valid
      (Actor|DestroyActor _returnvalue))
    (:Is%20Not%20Valid
      _))
  (Collision|SetCollisionEnabled (Variables|Default|GetBox) "NoCollision")
  (Components|Activation|Activate (Variables|Default|GetParticleSystem1) false)
  (Utilities|FlowControl|Delay 0.5)
  (Components|Activation|Activate (Variables|Default|GetParticleSystem2) false)
  (Utilities|FlowControl|Delay 0.5)
  (Components|Activation|Activate (Variables|Default|GetParticleSystem3) false)
  (Utilities|FlowControl|Delay 0.5)
  (Components|Activation|Activate (Variables|Default|GetParticleSystem4) false)
  (Utilities|FlowControl|Delay 0.5)
  (Components|Activation|Activate (Variables|Default|GetParticleSystem) false)
  (Utilities|FlowControl|Delay 0.5)
  (Components|Activation|Activate (Variables|Default|GetParticleSystem5) false)
  (Development|SetHiddeninGame (Variables|Default|GetStaticMesh) true false)
  (Utilities|FlowControl|Delay 2.0)
  (Game|OpenLevel(byObjectReference) "/Game/TitouanDev/Lv_Win.Lv_Win"))

(event Custom|SecondaryShot
  (if (not (Variables|Default|GetDead?))
    (if (Math|Random|RandomBool)
      (Game|SpawnActorfromClass "/Game/TitouanDev/Boss/BP_Boss2ndShotSpawner.BP_Boss2ndShotSpawner_C" (Transformation|GetWorldTransform (Variables|Default|GetRightCannon)) "Undefined" "MultiplyWithRoot" 0 0)
      (else
        (Game|SpawnActorfromClass "/Game/TitouanDev/Boss/BP_Boss2ndShotSpawner.BP_Boss2ndShotSpawner_C" (Transformation|GetWorldTransform (Variables|Default|GetLeftCannon)) "Undefined" "MultiplyWithRoot" 0 0)))))

(event Custom|Movement
  (bind _as_bp_main_chara (Variables|Default|GetAs%20BP%20Main%20Chara))
  (bind _returnvalue (Transformation|GetActorLocation _as_bp_main_chara))
  (bind _returnvalue_2 (+ (.y _returnvalue) 2.4e+03))
  (bind _movement (Timeline|Move PlayFromStart)
    (:Update
      (if (not (Variables|Default|GetDead?))
        (Transformation|SetActorLocation (Math|Vector|MakeVector (+ (* _movement 1.1e+03) 1.5e+03) _returnvalue_2 0.0) false false)
        (else
          (Transformation|SetActorLocation (Math|Vector|MakeVector (.x (Transformation|GetActorLocation)) _returnvalue_2 0.0) false false))))
    (:Finished
      (CallFunction|Movement))))

(event Custom|Activate
  (Variables|Default|SetActivated? true)
  (Game|SpawnActorfromClass "/Game/TitouanDev/Boss/BP_BossLaser.BP_BossLaser_C" (Math|Transform|MakeTransform "0, 0, 0" "0, 0, 0" "1.000000,1.000000,1.000000") "Undefined" "MultiplyWithRoot" 0 0)
  (bind _returnvalue (UserInterface|CreateWidget "/Game/TitouanDev/Boss/UI_BossHealth.UI_BossHealth_C"))
  (bind _output_get (Variables|Default|SetUI_Ref _returnvalue))
  (UserInterface|Viewport|AddtoViewport _output_get 0)
  (Utilities|Time|SetTimerbyEvent (delegate Custom|SecondaryShot) 0.6 true)
  (CallFunction|Movement))

(event EventTick
  (params (DeltaSeconds :type Float%20%28single-precision%29))
  (if (not (Variables|Default|GetActivated?))
    (if (<= (Math|Vector|VectorLength (- (Transformation|GetActorLocation (Variables|Default|GetAs%20BP%20Main%20Chara)) (Transformation|GetActorLocation))) 2.4e+03)
      (CallFunction|Activate))))

(event EventBeginPlay
  (bind _asbp_main_chara (Utilities|Casting|CastToBP_MainChara (Game|GetPlayerCharacter 0)))
  (Variables|Default|SetAs%20BP%20Main%20Chara _asbp_main_chara))

(event Collision|EventActorBeginOverlap
  (params (OtherActor :type Actor%20Object%20Reference))
  (bind _asbp_main_chara (Utilities|Casting|CastToBP_MainChara OtherActor))
  (Game|Damage|ApplyDamage _asbp_main_chara 5.0 0 0))

(event Game|Damage|EventAnyDamage
  (params (Damage :type Float%20%28single-precision%29) (DamageType :type Damage%20Type%20Object%20Reference) (InstigatedBy :type Controller%20Object%20Reference) (DamageCauser :type Actor%20Object%20Reference))
  (if (and (Variables|Default|GetActivated?) (not (Variables|Default|GetDead?)))
    (bind _output_get (Variables|Default|SetLife (- (Variables|Default|GetLife) Damage)))
    (if (<= _output_get 0.0)
      (Utilities|FlowControl|DoOnce false
        (:Completed
          (CallFunction|Death))))))

(fn ConstructionScript)