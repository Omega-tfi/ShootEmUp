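; BP_HealPellet is a pickup that heals BP_MainChara on overlap with its Sphere1 component.
; It adds a fixed amount to Life; the max-life comparison is unconnected and the select always takes the increased value, so Life can exceed MaxLife.
; It then plays a heal sound, clears the DidNotHealLikeaLOSER flag on BP_TopDownGameMode and destroys itself.
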(event OnComponentBeginOverlap(Sphere1)
  (params (OverlappedComponent :type Primitive%20Component%20Object%20Reference) (OtherActor :type Actor%20Object%20Reference) (OtherComp :type Primitive%20Component%20Object%20Reference) (OtherBodyIndex :type Integer) (bFromSweep :type Boolean) (SweepResult :type Hit%20Result%20Structure%20%28by%20ref%29))
  (bind _asbp_main_chara (Utilities|Casting|CastToBP_MainChara OtherActor))
  (Variables|/Game/TitouanDev/BP_MainChara.BP_MainChara_C|SetLife _asbp_main_chara (Math|Float|SelectFloat (Variables|/Game/TitouanDev/BP_MainChara.BP_MainChara_C|GetMaxLife _asbp_main_chara) (+ (Variables|/Game/TitouanDev/BP_MainChara.BP_MainChara_C|GetLife _asbp_main_chara) 3.0) false))
  (Audio|PlaySound2D "/Game/GuillaumeDev/SoundEffects/Cues/Cue_Heal.Cue_Heal" 1.0 1.0 0.0 0 0)
  (bind _asbp_top_down_game_mode (Utilities|Casting|CastToBP_TopDownGameMode (Game|GetGameMode)))
  (Variables|/Game/TopDown/Blueprints/BP_TopDownGameMode.BP_TopDownGameMode_C|SetDidNotHealLikeaLOSER _asbp_top_down_game_mode false)
  (Actor|DestroyActor))

(event EventBeginPlay)

(event Collision|EventActorBeginOverlap
  (params (OtherActor :type Actor%20Object%20Reference)))

(event EventTick
  (params (DeltaSeconds :type Float%20%28single-precision%29)))

(fn ConstructionScript)