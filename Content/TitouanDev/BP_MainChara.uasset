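; Player ship for a shoot 'em up, which scrolls forward constantly along Y and fires automatically.
; Two looping timers spawn angled main shots and faster secondary shot spawners from paired cannons until death, and a health widget is created at start.
; Damage grants brief invincibility, then rechecks overlaps to reapply boss or laser contact damage.
; At zero life the ship stops firing, disables collision and spawns an explosion once.
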(event Custom|MainShoot
  (if (not (Variables|Default|GetIsDead?))
    (Game|SpawnActorfromClass "/Game/TitouanDev/BP_MainShot.BP_MainShot_C" (Math|Transform|MakeTransform (Transformation|GetWorldLocation (Variables|Default|GetMainCannonLeft)) "0.000000,-5.000000,0.000000" "1.000000,1.000000,1.000000") "AlwaysSpawn" "MultiplyWithRoot" 0 0)
    (Game|SpawnActorfromClass "/Game/TitouanDev/BP_MainShot.BP_MainShot_C" (Math|Transform|MakeTransform (Transformation|GetWorldLocation (Variables|Default|GetMainCannonRight)) "0.000000,5.000000,0.000000" "1.000000,1.000000,1.000000") "AlwaysSpawn" "MultiplyWithRoot" 0 0)
    (Audio|PlaySound2D "/Game/SFX/SoundCues/SC_MainShot.SC_MainShot" 0.1 1.0 0.0 0 0)))

(event Custom|SecondaryShot
  (if (not (Variables|Default|GetIsDead?))
    (Game|SpawnActorfromClass "/Game/TitouanDev/BP_2ndShotSpawner.BP_2ndShotSpawner_C" (Transformation|GetWorldTransform (Variables|Default|GetSecondCannonLeft)) "AlwaysSpawn" "MultiplyWithRoot" 0 0)
    (Game|SpawnActorfromClass "/Game/TitouanDev/BP_2ndShotSpawner.BP_2ndShotSpawner_C" (Transformation|GetWorldTransform (Variables|Default|GetSecondCannonRight)) "AlwaysSpawn" "MultiplyWithRoot" 0 0)
    (Audio|PlaySound2D "/Game/SFX/SoundCues/SC_SecondaryShot.SC_SecondaryShot" 0.1 1.0 0.0 0 0)))

(event EventBeginPlay
  (Utilities|Time|SetTimerbyEvent (delegate Custom|MainShoot) 1.0 true)
  (Utilities|Time|SetTimerbyEvent (delegate Custom|SecondaryShot) 0.3 true)
  (bind _returnvalue (UserInterface|CreateWidget "/Game/TitouanDev/UI_Health.UI_Health_C"))
  (bind _output_get (Variables|Default|SetHealthUIRef _returnvalue))
  (UserInterface|Viewport|AddtoViewport _output_get 0))

(event EventTick
  (params (DeltaSeconds :type Float%20%28single-precision%29))
  (Transformation|AddActorWorldOffset (Math|Vector|MakeVector 0.0 (* DeltaSeconds 5e+02) 0.0)))

(event Game|Damage|EventAnyDamage
  (params (Damage :type Float%20%28single-precision%29) (DamageType :type Damage%20Type%20Object%20Reference) (InstigatedBy :type Controller%20Object%20Reference) (DamageCauser :type Actor%20Object%20Reference))
  (if (not (Variables|Default|GetInvincible?))
    (bind _output_get (Variables|Default|SetLife (- (Variables|Default|GetLife) Damage)))
    (if (<= _output_get 0.0)
      (Utilities|FlowControl|DoOnce false
        (:Completed
          (Variables|Default|SetIsDead? true)
          (Collision|SetCollisionEnabled (Variables|Default|GetBox) "NoCollision")
          (Game|SpawnActorfromClass "/Game/TitouanDev/BP_DeathExplosion.BP_DeathExplosion_C" (Transformation|GetWorldTransform (Variables|Default|GetShip)) "Undefined" "MultiplyWithRoot" 0 0)))
      (else
        (Variables|Default|SetInvincible? true)
        (Utilities|FlowControl|Delay 0.5)
        (Variables|Default|SetInvincible? false)
        (for _array_element (Collision|GetOverlappingActors 0 :!class /Script/Engine.Actor)
          (Utilities|Casting|CastToBP_BossLaser _array_element
            (:then
              (Game|Damage|ApplyDamage 0 3.0 0 0))
            (:CastFailed
              (Utilities|Casting|CastToBP_Boss _array_element)
              (Game|Damage|ApplyDamage 0 5.0 0 0))))))))

(fn ConstructionScript)