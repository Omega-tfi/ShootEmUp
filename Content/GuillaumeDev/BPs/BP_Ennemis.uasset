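; Enemy spaceship that fires at the player ship, sometimes with random offset, and deals damage on overlap.
; BeginPlay randomly picks material and movement: straight down -Y, rush at a snapshot of the player's position, or timeline-driven zigzag.
; Looping timers appear to drive shooting and despawning once far behind the player.
; Death spawns an explosion and increments the GameMode counter; construction sets the mesh from SpaceshipType, separate from the random movement.
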(event Custom|Moving
  (Utilities|Time|SetTimerbyEvent (Utilities|Select :Index (Variables|Movements|GetMovementOption) :Option%200 (EventDispatchers|CreateEvent :!event Custom|MovementOption1) :Option%201 (EventDispatchers|CreateEvent :!event Custom|MovementOption2) :Option%202 (EventDispatchers|CreateEvent :!event Custom|MovementOption3)) 0.1))

(event Custom|Shot%20Event
  (bind _returnvalue (Transformation|GetActorLocation))
  (bind _playerref (Variables|References|GetPlayerRef))
  (bind _arrow (Variables|Default|GetArrow))
  (bind _returnvalue_2 (Transformation|GetWorldTransform _arrow))
  (bind _ship (Variables|/Game/TitouanDev/BP_MainChara.BP_MainChara_C|GetShip _playerref))
  (bind _returnvalue_3 (Transformation|GetWorldLocation _ship))
  ;[1 1 1] Shooting is easy lmao
  (Game|SpawnActorfromClass "/Game/GuillaumeDev/BPs/BP_Balle_Ennemi.BP_Balle_Ennemi_C" (Math|Transform|SelectTransform (Math|Transform|MakeTransform (.location _returnvalue_2) (Math|Rotator|FindLookatRotation _returnvalue _returnvalue_3) (.scale _returnvalue_2)) (Math|Transform|MakeTransform (.location _returnvalue_2) (Math|Rotator|FindLookatRotation _returnvalue (+ _returnvalue_3 (Math|Vector|MakeVector 0.0 (Math|Random|RandomFloatinRange -5e+01 5e+01) 0.0))) (.scale _returnvalue_2)) (Math|Random|RandomBool)) "Undefined" "MultiplyWithRoot" 0 0))

(event Custom|MovementOption3
  (bind _spawnlocation (Variables|Movements|GetSpawnLocation))
  (Variables|Movements-Mov3|SetLerpStart (Math|Float|Absolute(Float) (- (/ (.x _spawnlocation) 3e+03) 1.0)))
  (Variables|Movements-Mov3|SetCurrentYPosition (+ (- (.y _spawnlocation) 2e+03) (/ 2e+03 (Variables|Movements-Mov3|GetLerpStart))))
  (Utilities|FlowControl|Sequence
    (:then_0
      (bind _newtrack_2 (Timeline|Timeline%200%20to%201%20%20with%203 SetNewTime)
        (:Update
          (Transformation|SetActorLocation (Math|Vector|MakeVector (Math|Float|Lerp 1.5e+02 2.85e+03 _newtrack_2) (Math|Float|Lerp (Variables|Movements-Mov3|GetCurrentYPosition) (- (Variables|Movements-Mov3|GetCurrentYPosition) 1.5e+03) _newtrack_2) (.z (Variables|Movements|GetSpawnLocation))) false false))
        (:Finished
          (Variables|Movements-Mov3|SetCurrentYPosition (- (Variables|Movements-Mov3|GetCurrentYPosition) 1.5e+03))
          (CallFunction|3:FromEnd)
          (Transformation|SetActorRotation "0.000000,-45.000000,0.000000")
          (Utilities|FlowControl|DoOnce false
            (:Completed
              (Variables|Movements-Mov3|SetLerpStart 0.0))))))
    (:then_1
      (Timeline|Timeline%200%20to%201%20%20with%203 Play))))

(event Custom|MovementOption1
  (bind _spawnlocation (Variables|Movements|GetSpawnLocation))
  ;[1 1 1] SimpleMovement
  (bind _newtrack_0 (Timeline|0%20to%201%20numbah%201 PlayFromStart)
    (:Update
      (Transformation|SetActorLocation (Math|Vector|MakeVector (.x _spawnlocation) (+ (Math|Float|Lerp 0.0 -6e+03 _newtrack_0) (.y _spawnlocation)) (.z _spawnlocation)) false false))))

(event Custom|MovementOption2
  (bind _playerref (Variables|References|GetPlayerRef))
  (bind _spawnlocation (Variables|Movements|GetSpawnLocation))
  (bind _ship (Variables|/Game/TitouanDev/BP_MainChara.BP_MainChara_C|GetShip _playerref))
  (bind _returnvalue (Transformation|GetWorldLocation _ship))
  (bind _returnvalue_2 (Math|Rotator|FindLookatRotation _returnvalue _spawnlocation))
  ;[1 1 1] PlayerRush
  (Variables|Movements-Mov3|SetPlayerLocSnapshot _returnvalue)
  (Transformation|SetActorRotation (Math|Rotator|MakeRotator (.roll _returnvalue_2) (.pitch _returnvalue_2) (- (.yaw _returnvalue_2) 9e+01)))
  (bind _newtrack_0 (Timeline|0%20to%201%20Numero%202 PlayFromStart)
    (:Update
      (Transformation|SetActorLocation (Math|Vector|Lerp(Vector) (Variables|Movements|GetSpawnLocation) (Variables|Movements-Mov3|GetPlayerLocSnapshot) _newtrack_0) false false))))

(event Custom|Is%20Ship%20Too%20Far?
  (if (< (.y (Transformation|GetActorLocation)) (- (.y (Transformation|GetWorldLocation (Variables|/Script/Engine.Character|GetCapsuleComponent (Variables|References|GetPlayerRef)))) 3e+03))
    (Actor|DestroyActor)))

(event Custom|3:FromStart
  (Variables|Movements-Mov3|SetCurrentYPosition (.y (Transformation|GetWorldLocation (Variables|Default|GetStaticMesh))))
  (bind _newtrack_2 (Timeline|Timeline%200%20to%201%20%20with%203 PlayFromStart)
    (:Update
      (Transformation|SetActorLocation (Math|Vector|MakeVector (Math|Float|Lerp 1.5e+02 2.85e+03 _newtrack_2) (Math|Float|Lerp (Variables|Movements-Mov3|GetCurrentYPosition) (- (Variables|Movements-Mov3|GetCurrentYPosition) 1.5e+03) _newtrack_2) (.z (Variables|Movements|GetSpawnLocation))) false false))
    (:Finished
      (Variables|Movements-Mov3|SetCurrentYPosition (- (Variables|Movements-Mov3|GetCurrentYPosition) 1.5e+03))
      (CallFunction|3:FromEnd)
      (Transformation|SetActorRotation "0.000000,-45.000000,0.000000")
      (Utilities|FlowControl|DoOnce false
        (:Completed
          (Variables|Movements-Mov3|SetLerpStart 0.0))))))

(event Custom|3:FromEnd
  (Variables|Movements-Mov3|SetCurrentYPosition (.y (Transformation|GetWorldLocation (Variables|Default|GetStaticMesh))))
  (bind _newtrack_0 (Timeline|Timeline%200%20to%201%20second%20third PlayFromStart)
    (:Update
      (Transformation|SetActorLocation (Math|Vector|MakeVector (Math|Float|Lerp 2.85e+03 1.5e+02 _newtrack_0) (Math|Float|Lerp (Variables|Movements-Mov3|GetCurrentYPosition) (- (Variables|Movements-Mov3|GetCurrentYPosition) 1.5e+03) _newtrack_0) (.z (Variables|Movements|GetSpawnLocation))) false false))
    (:Finished
      (Variables|Movements-Mov3|SetCurrentYPosition (- (Variables|Movements-Mov3|GetCurrentYPosition) 1.5e+03))
      (CallFunction|3:FromStart)
      (Transformation|SetActorRotation "0.000000,45.000000,0.000000"))))

(event EventBeginPlay
  (bind _output_get (Variables|Movements|SetMovementOption (Math|Random|RandomIntegerinRange 0 2)))
  (Rendering|Material|SetMaterial (Variables|Default|GetStaticMesh) 0 (Utilities|Select :Index _output_get :Option%200 "/Game/SpaceShips/MI_NormalShip.MI_NormalShip" :Option%201 "/Game/SpaceShips/MI_BerserkShip.MI_BerserkShip" :Option%202 "/Game/SpaceShips/MI_DumbShip.MI_DumbShip"))
  (bind _asbp_main_chara (Utilities|Casting|CastToBP_MainChara (Game|GetPlayerCharacter 0)))
  (Variables|References|SetPlayerRef _asbp_main_chara)
  (Utilities|Time|SetTimerbyEvent (EventDispatchers|CreateEvent :!event Custom|Shot%20Event) 1.5 true)
  (Variables|Movements|SetSpawnLocation (Transformation|GetWorldLocation (Variables|Default|GetStaticMesh)))
  (CallFunction|Moving)
  (Utilities|Time|SetTimerbyEvent (EventDispatchers|CreateEvent :!event Custom|Is%20Ship%20Too%20Far?) 1.0 true))

(event Collision|EventActorBeginOverlap
  (params (OtherActor :type Actor%20Object%20Reference))
  (bind _asbp_main_chara (Utilities|Casting|CastToBP_MainChara OtherActor))
  (Game|Damage|ApplyDamage _asbp_main_chara 2.0 0 0))

(event Game|Damage|EventAnyDamage
  (params (Damage :type Float%20%28single-precision%29) (DamageType :type Damage%20Type%20Object%20Reference) (InstigatedBy :type Controller%20Object%20Reference) (DamageCauser :type Actor%20Object%20Reference))
  (Variables|Stats|SetHPs (- (Variables|Stats|GetHPs) Damage))
  (if (<= (Variables|Stats|GetHPs) 0.0)
    (Game|SpawnActorfromClass "/Game/TitouanDev/BP_MainShotExplosion.BP_MainShotExplosion_C" (Transformation|GetActorTransform) "Undefined" "MultiplyWithRoot" 0 0)
    (Actor|DestroyActor)
    (bind _asbp_top_down_game_mode (Utilities|Casting|CastToBP_TopDownGameMode (Game|GetGameMode)))
    (Default|IncrementCounter _asbp_top_down_game_mode)))

(fn ConstructionScript
  (Components|StaticMesh|SetStaticMesh (Variables|Default|GetStaticMesh) (Utilities|Select :Index (Variables|Default|GetSpaceship%20Type) :NewEnumerator0 "/Game/SpaceShips/Spaceship4.Spaceship4" :NewEnumerator1 "/Game/SpaceShips/Spaceship2.Spaceship2" :NewEnumerator2 "/Game/SpaceShips/Spaceship5.Spaceship5")))